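; BP_EnemyBase is a base enemy Blueprint that takes hit damage and hands ammo to its attacker once dead.
; HitDamage applies damage, then an IsDead macro gates ammo refills while CanDropAmmo is set and destroys the actor otherwise.
; RefillPlayerAmmoBP looks up Hits in DropPosition for a key into Drops and refills the initiator.
; A missing Hits entry clears CanDropAmmo, so a later hit destroys the dead enemy.
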(event `/Game/Interfaces/BI_Enemy.HitDamage`
  (params (Damage :type "Float (double-precision)") (Initiator :type "/Game/FirstPerson/Blueprints/BP_LightGunShooterPlayer Object Reference"))
  (`self.TakeDamage` Damage)
  (`self.IsDeadMacro`
    (:`True`
      (if (`self.CanDropAmmo`)
        (`self.Refill Player AmmoBP` Initiator)
        (else
          (`self.K2_DestroyActor`))))))

(fn `Refill Player AmmoBP`
  (params (PlayerCharacter :type "LightGunShooterPlayer Object Reference"))
  (bind (_value _returnvalue) (`BlueprintMapLibrary.Map_Find` (`self.DropPosition`) (`self.Hits`)))
  (if _returnvalue
    (`LightGunShooterPlayer.Refill` PlayerCharacter _value (`BlueprintMapLibrary.Map_Find` (`self.Drops`) _value))
    (else
      (set `self.CanDropAmmo` false))))

(fn `UserConstructionScript`)